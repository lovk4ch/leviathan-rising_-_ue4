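; BP_Spawner lays out a grid of instanced static meshes and feeds the player's location to the Pintable material parameters.
; On BeginPlay it adds rows of instances at 100-unit steps along X, then recursively calls Redraw, stepping along negative Y until the Columns counter runs out.
; Every Tick it writes the player pawn's location to the Position vector in the Pintable_Params material parameter collection.
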(event `Redraw`
  (bind (_returnvalue_x _returnvalue_y _returnvalue_z) (`KismetMathLibrary.BreakVector` (`SceneComponent.K2_GetComponentLocation` (`self.DefaultSceneRoot`))))
  (for _ (range (+ (`self.Rows`) 1)) :!label _label
    (`InstancedStaticMeshComponent.AddInstance` (`self.InstancedStaticMesh`) (`KismetMathLibrary.MakeTransform` (`self.Next`)))
    (set `self.Next` (+ (* (`KismetMathLibrary.GetForwardVector` (struct)) 100.0) (`self.Next`))))
  (bind _output_get (set `self.Front` (+ (* (`KismetMathLibrary.GetRightVector` (struct)) -100.0) (`self.Front`))))
  (set `self.Next` (`KismetMathLibrary.MakeVector` _returnvalue_x (.y _output_get) _returnvalue_z))
  (bind _result (`/Engine/EditorBlueprintResources/StandardMacros.DecrementInt` (`self.Columns`))
    (:`  `
      (if (>= _result 1)
        (`self.Redraw`)))))

(event `self.ReceiveBeginPlay`
  (bind (_front_x _front_y) (`KismetMathLibrary.BreakVector` (`self.Front`)))
  (bind (_returnvalue_x _returnvalue_y _returnvalue_z) (`KismetMathLibrary.BreakVector` (`SceneComponent.K2_GetComponentLocation` (`self.DefaultSceneRoot`))))
  (set `self.Next` (`KismetMathLibrary.MakeVector` _returnvalue_x _front_y _returnvalue_z))
  (goto _label))

(event `self.ReceiveTick`
  (params (DeltaSeconds :type "Float (single-precision)"))
  (`KismetMaterialLibrary.SetVectorParameterValue` "/Game/Materials/lovk4ch/Pintable/Pintable_Params.Pintable_Params" "Position" (`KismetMathLibrary.Conv_VectorToLinearColor` (`self.K2_GetActorLocation` (`GameplayStatics.GetPlayerPawn` 0)))))

(fn `UserConstructionScript`)